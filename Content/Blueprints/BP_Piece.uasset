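; BP_Piece is a piece in quantum checkers, with color, king state and a probability read from BP_Board.
; Tick updates its visuals and probability label, destroying the piece at zero probability.
; On the owner's turn, left-click traces diagonals to spawn move, capture or measurement markers, while right-click spawns quantum moves on empty squares.
; Kings also trace backward, and ChainTrace continues captures in one direction or passes the turn.
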(event `self.ReceiveBeginPlay`
  ;[1 1 1] Get character reference
  (bind _asplayer_ (cast `/Game/Blueprints/GlobalBP/Player+` (`GameplayStatics.GetPlayerCharacter` 0)))
  (set `self.Character` _asplayer_)
  ;[1 1 1] Get Board reference
  (bind _outactors (`GameplayStatics.GetAllActorsOfClass` "/Game/Blueprints/BP_Board.BP_Board_C"))
  (bind _output (`|GetArrayItem` _outactors))
  (if (`KismetSystemLibrary.IsValid` _output)
    (set `self.Board` _output)))

(event `self.ReceiveTick`
  (params (DeltaSeconds :type "Float (single-precision)"))
  (bind (_returnvalue_x _returnvalue_y) (`KismetMathLibrary.BreakVector` (`self.K2_GetActorLocation`)))
  (bind _character (`self.Character`))
  (bind _prob (`self.Prob`))
  ;[1 1 1] Set rotation
  (`self.K2_SetActorRelativeRotation` (select `/Game/Blueprints/Enums/PieceColor` (`self.Piece Color`) :`NewEnumerator4` (struct :`Yaw` 180.0) :!type "Rotator Structure"))
  ;[1 1 1] Set type
  (`SceneComponent.SetVisibility` (`self.KingsCross`) (select `/Game/Blueprints/Enums/PieceType` (`self.Piece Type`) :`NewEnumerator5` true) true)
  ;[1 1 1] Set selection particle
  (`SceneComponent.SetVisibility` (`self.SelectionHighlight`) (== (`/Game/Blueprints/GlobalBP/Player+.Selected Piece` _character) self) true)
  ;[1 1 1] Set probability Text
  (bind _qubit (`/Game/Blueprints/GlobalBP/Player+.Get Qubit` _character _returnvalue_x _returnvalue_y))
  (bind _output_get (set `self.Probability` (`KismetStringLibrary.Conv_StringToDouble` (`|GetArrayItem` (`/Game/Blueprints/BP_Board.Probability Strings` (`self.Board`)) _qubit))))
  (`TextRenderComponent.K2_SetText` _prob (select `bool` (`/Game/Blueprints/GlobalBP/Player+.Percentage` (`self.Character`)) :`false` (`KismetTextLibrary.Conv_DoubleToText` _output_get "HalfToEven" false true 1 324 0 5) :`true` (`KismetTextLibrary.Conv_StringToText` (`KismetStringLibrary.Concat_StrStr` (`KismetTextLibrary.Conv_TextToString` (`KismetTextLibrary.Conv_DoubleToText` (* _output_get 100.0) "HalfToEven" false true 1 324 0 5)) "%"))))
  (`SceneComponent.K2_SetWorldRotation` _prob (`KismetMathLibrary.FindLookAtRotation` (`self.K2_GetActorLocation`) (`self.K2_GetActorLocation` (`self.Character`))) false false)
  (if (== (`self.Probability`) 0.0)
    (if (`KismetSystemLibrary.IsValid` self)
      (`self.K2_DestroyActor`))))

(event `Quantum Trace`
  (`self.DiagonalTrace_Quantum` 1.0 1.0 self
    (:`true`
      (`self.DiagonalTrace_Quantum` 1.0 -1.0 self "NewEnumerator1"
        (:`true`
          (if (`|EnumEquality` (`self.Piece Type`) "NewEnumerator5")
            (`self.DiagonalTrace_Quantum` -1.0 1.0 self "NewEnumerator2"
              (:`true`
                (`self.DiagonalTrace_Quantum` -1.0 -1.0 self "NewEnumerator3")))))))))

(event `Trace`
  (`self.DiagonalTrace` 1.0 1.0 self
    (:`true`
      (`self.DiagonalTrace` 1.0 -1.0 self "NewEnumerator1"
        (:`true`
          (if (`|EnumEquality` (`self.Piece Type`) "NewEnumerator5")
            (`self.DiagonalTrace` -1.0 1.0 self "NewEnumerator2"
              (:`true`
                (`self.DiagonalTrace` -1.0 -1.0 self "NewEnumerator3")))))))))

(event `self.ReceiveActorOnClicked`
  (params (ButtonPressed :type "Key Structure"))
  (bind _player_turn_white (`/Game/Blueprints/GlobalBP/Player+.Player Turn White` (`self.Character`)))
  (if (select `/Game/Blueprints/Enums/PieceColor` (`self.Piece Color`) :`NewEnumerator4` (not _player_turn_white) :`NewEnumerator5` _player_turn_white)
    (bind _selected (`/Game/Blueprints/GlobalBP/Player+.Set Selected Piece` (`self.Character`) self))
    (if _selected
      (if (== ButtonPressed "LeftMouseButton")
        (`self.Trace` :!label _label)
        (elif (== ButtonPressed "RightMouseButton")
          (`self.Quantum Trace`)
          (else
            (goto _label))))
      (`GameplayStatics.PlaySound2D` "/Engine/VREditor/Sounds/UI/Laser_Push.Laser_Push" 1.5 1.0 0.0 null null)
      (else
        (`GameplayStatics.PlaySound2D` "/Engine/VREditor/Sounds/UI/Laser_Pull.Laser_Pull" 1.5 1.0 0.0 null null)))))

(event `ChainTrace`
  (params (Direction :type "/Game/Blueprints/Enums/Direction Enum" :default "NewEnumerator0"))
  (bind (_x _y) (`KismetMathLibrary.BreakVector2D` (select `/Game/Blueprints/Enums/Direction` Direction :`NewEnumerator0` (1.0 1.0) :`NewEnumerator1` (1.0 -1.0) :`NewEnumerator2` (-1.0 1.0) :`NewEnumerator3` (-1.0 -1.0) :!type "Vector2D Structure")))
  (`/Game/Blueprints/BP_Board.Get Prob` (`self.Board`))
  (set `self.ChainCapture` true)
  (`self.DiagonalTrace` _x _y self Direction))

(event `self.ReceiveActorBeginOverlap`
  (params (OtherActor :type "Actor Object Reference"))
  (bind _asbp_piece (cast `/Game/Blueprints/BP_Piece` OtherActor))
  (if (== (`/Game/Blueprints/BP_Piece.Probability` _asbp_piece) 0.0)
    (if (`KismetSystemLibrary.IsValid` _asbp_piece)
      (`self.K2_DestroyActor`))))

(fn `UserConstructionScript`
  (bind _piece_materials (`self.Piece Materials`))
  (`PrimitiveComponent.SetMaterial` (`self.Piece`) 0 (select `/Game/Blueprints/Enums/PieceColor` (`self.Piece Color`) :`NewEnumerator4` (`|GetArrayItem` _piece_materials) :`NewEnumerator5` (`|GetArrayItem` _piece_materials 1)))
  (`self.K2_SetActorRelativeRotation` (select `/Game/Blueprints/Enums/PieceColor` (`self.Piece Color`) :`NewEnumerator4` (struct :`Yaw` 180.0) :!type "Rotator Structure"))
  (`SceneComponent.SetVisibility` (`self.KingsCross`) (select `/Game/Blueprints/Enums/PieceType` (`self.Piece Type`) :`NewEnumerator5` true) true)
  (`PrimitiveComponent.SetMaterial` (`self.KingsCross`) 0 (select `/Game/Blueprints/Enums/PieceColor` (`self.Piece Color`) :`NewEnumerator4` "/Game/StarterContent/Materials/M_GBlack.M_GBlack" :`NewEnumerator5` "/Game/StarterContent/Materials/M_GWhite.M_GWhite" :!type "MaterialInterface Object Reference"))
  (set `self.Tags` (`|MakeArray` (select `/Game/Blueprints/Enums/PieceColor` (`self.Piece Color`) :`NewEnumerator4` "Black" :`NewEnumerator5` "White" :!type "Name"))))