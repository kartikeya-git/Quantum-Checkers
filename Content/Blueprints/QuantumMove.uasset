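; Clickable move marker that performs a quantum move for the player's selected piece in a board game.
; On click, it converts the piece's and its own locations to qubits, sets them as BP_Board's source and target, and runs QuantumMove.
; It then spawns a copy of the piece on itself, calls GetProb and changes turns.
; It destroys itself on overlap, or at construction if a short downward trace hits nothing.
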(event `self.ReceiveBeginPlay`
  (bind _asplayer_ (cast `/Game/Blueprints/GlobalBP/Player+` (`GameplayStatics.GetPlayerCharacter` 0)))
  (set `self.Character` _asplayer_)
  (bind _outactors (`GameplayStatics.GetAllActorsOfClass` "/Game/Blueprints/BP_Board.BP_Board_C"))
  (bind _output (`|GetArrayItem` _outactors))
  (if (`KismetSystemLibrary.IsValid` _output)
    (set `self.Board` _output)))

(event `self.ReceiveActorOnClicked`
  (params (ButtonPressed :type "Key Structure"))
  (bind (_returnvalue_x _returnvalue_y) (`KismetMathLibrary.BreakVector` (`self.K2_GetActorLocation`)))
  (bind _board (`self.Board`))
  (bind _selected_piece (`/Game/Blueprints/GlobalBP/Player+.Selected Piece` (`self.Character`)))
  (bind (_returnvalue_x_2 _returnvalue_y_2) (`KismetMathLibrary.BreakVector` (`self.K2_GetActorLocation` (`/Game/Blueprints/GlobalBP/Player+.Selected Piece` (`self.Character`)))))
  (`GameplayStatics.PlaySound2D` "/Engine/VREditor/Sounds/UI/Object_PickUp.Object_PickUp" 1.0 1.0 0.0 null null)
  (bind _qubit (`/Game/Blueprints/GlobalBP/Player+.Get Qubit` (`self.Character`) _returnvalue_x_2 _returnvalue_y_2))
  (set `/Game/Blueprints/BP_Board.Source` _qubit (`self.Board`))
  (bind _qubit_2 (`/Game/Blueprints/GlobalBP/Player+.Get Qubit` (`self.Character`) _returnvalue_x _returnvalue_y))
  (bind _output_get (set `/Game/Blueprints/BP_Board.Target` _qubit_2 _board))
  (`/Game/Blueprints/BP_Board.Quantum Move` _board)
  (`|SpawnActorFromClass` "/Game/Blueprints/BP_Piece.BP_Piece_C" (`KismetMathLibrary.MakeTransform` (`KismetMathLibrary.MakeVector` _returnvalue_x _returnvalue_y 60.0)) "Undefined" "OverrideRootScale" null (`/Game/Blueprints/BP_Piece.Piece Color` _selected_piece) (`/Game/Blueprints/BP_Piece.Piece Type` _selected_piece) (`/Game/Blueprints/BP_Piece.Piece Number` _selected_piece) null)
  (`/Game/Blueprints/BP_Board.Get Prob` (`self.Board`))
  (`/Game/Blueprints/GlobalBP/Player+.ChangeTurns` (`self.Character`)))

(event `self.ReceiveActorBeginOverlap`
  (params (OtherActor :type "Actor Object Reference"))
  (if (`KismetSystemLibrary.IsValid` self)
    (`self.K2_DestroyActor`)))

(fn `UserConstructionScript`
  (bind _returnvalue (`self.K2_GetActorLocation`))
  (bind (_outhit _returnvalue_2) (`KismetSystemLibrary.LineTraceSingle` _returnvalue (+ _returnvalue (* (`self.GetActorUpVector`) -50.0)) "TraceTypeQuery1"))
  (if _returnvalue_2
    _
    (elif (`KismetSystemLibrary.IsValid` self)
      (`self.K2_DestroyActor`))))