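; BP_Board is a board actor that bridges Blueprint to a Python component for qubit-based gameplay with normal and quantum moves.
; On BeginPlay it caches the player character and fetches the initial probability strings from Python.
; Its events call Python methods by name for moves, measurement and two qubit resets, storing probability and boolean measurement results in variables.
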(event `self.ReceiveBeginPlay`
  (bind _asplayer_ (cast `/Game/Blueprints/GlobalBP/Player+` (`GameplayStatics.GetPlayerCharacter` 0)))
  (set `self.Character` _asplayer_)
  (`self.Get Prob`))

(event `Normal Move`
  (`PythonComponent.CallPythonComponentMethod` (`self.Python`) "normal_move" "")
  (`KismetSystemLibrary.PrintString` "Normal Move"))

(event `Get Prob`
  (bind _output_strings (`PythonComponent.CallPythonComponentMethodStringArray` (`self.Python`) "get_probability" ""))
  (set `self.Probability Strings` _output_strings))

(event `Quantum Move`
  (`PythonComponent.CallPythonComponentMethod` (`self.Python`) "quantumm_move" "")
  (`KismetSystemLibrary.PrintString` "Quantum Move"))

(event `Measurement`
  (bind _returnvalue (`PythonComponent.CallPythonComponentMethodBool` (`self.Python`) "measure" ""))
  (set `self.MeasurementResult` _returnvalue))

(event `Reset Qubit`
  (`PythonComponent.CallPythonComponentMethod` (`self.Python`) "reset_qubit" ""))

(event `Reset Qubit1`
  (`PythonComponent.CallPythonComponentMethod` (`self.Python`) "reset_qubit1" ""))

(fn `UserConstructionScript`)