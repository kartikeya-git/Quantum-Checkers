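; Clickable move-target marker for a quantum board game, destroying itself on overlap or when no surface lies beneath it.
; Clicking converts board positions to qubits for BP_Board's NormalMove, relocates the player's selected piece and changes turns.
; A specific piece type reaching its color's far row promotes with lightning effects.
; If that piece's probability is below one, a measurement decides first, and failure forfeits the move.
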(event `self.ReceiveActorBeginOverlap`
  (params (OtherActor :type "Actor Object Reference"))
  (if (`KismetSystemLibrary.IsValid` self)
    (`self.K2_DestroyActor`)))

(event `self.ReceiveBeginPlay`
  (bind _asplayer_ (cast `/Game/Blueprints/GlobalBP/Player+` (`GameplayStatics.GetPlayerCharacter` 0)))
  (set `self.Character` _asplayer_)
  (bind _outactors (`GameplayStatics.GetAllActorsOfClass` "/Game/Blueprints/BP_Board.BP_Board_C"))
  (bind _output (`|GetArrayItem` _outactors))
  (if (`KismetSystemLibrary.IsValid` _output)
    (set `self.Board` _output)))

(event `self.ReceiveActorOnClicked`
  (params (ButtonPressed :type "Key Structure"))
  (bind _returnvalue_x (`KismetMathLibrary.BreakVector` (`self.K2_GetActorLocation`)))
  (bind _returnvalue (`self.K2_GetActorLocation`))
  (bind (_returnvalue_x_2 _returnvalue_y) (`KismetMathLibrary.BreakVector` (`self.K2_GetActorLocation`)))
  (bind _board (`self.Board`))
  (bind _board_2 (`self.Board`))
  (bind _selected_piece (`/Game/Blueprints/GlobalBP/Player+.Selected Piece` (`self.Character`)))
  (bind (_returnvalue_x_3 _returnvalue_y_2) (`KismetMathLibrary.BreakVector` (`self.K2_GetActorLocation` _selected_piece)))
  (bind (_returnvalue_x_4 _returnvalue_y_3) (`KismetMathLibrary.BreakVector` (`self.K2_GetActorLocation` _selected_piece)))
  (`GameplayStatics.PlaySound2D` "/Engine/VREditor/Sounds/VR_ungrab.VR_ungrab" 1.0 1.0 0.0 null null)
  (if (`|EnumEquality` (`/Game/Blueprints/BP_Piece.Piece Type` _selected_piece) "NewEnumerator4")
    (if (`KismetMathLibrary.NearlyEqual_FloatFloat` (select `/Game/Blueprints/Enums/PieceColor` (`/Game/Blueprints/BP_Piece.Piece Color` _selected_piece) :`NewEnumerator5` 700.0 :!type "Float (single-precision)") _returnvalue_x 0.1)
      (if (`KismetMathLibrary.NearlyEqual_FloatFloat` (`/Game/Blueprints/BP_Piece.Probability` _selected_piece) 1.0 0.001)
        (`GameplayStatics.PlaySound2D` "/Engine/VREditor/Sounds/UI/Enter_Simulate.Enter_Simulate" 1.0 1.0 0.0 null null :!label _label)
        (`GameplayStatics.SpawnEmitterAtLocation` "/Game/FXVarietyPack/Particles/P_ky_lightning3.P_ky_lightning3" _returnvalue)
        (`GameplayStatics.SpawnEmitterAtLocation` "/Game/FXVarietyPack/Particles/P_ky_lightning1.P_ky_lightning1" _returnvalue)
        (`GameplayStatics.SpawnEmitterAtLocation` "/Game/FXVarietyPack/Particles/P_ky_lightning2.P_ky_lightning2" _returnvalue)
        (set `/Game/Blueprints/BP_Piece.Piece Type` "NewEnumerator5" _selected_piece)
        (bind _qubit (`/Game/Blueprints/GlobalBP/Player+.Get Qubit` (`self.Character`) _returnvalue_x_4 _returnvalue_y_3 :!label _label_2))
        (set `/Game/Blueprints/BP_Board.Source` _qubit (`self.Board`))
        (bind _qubit_2 (`/Game/Blueprints/GlobalBP/Player+.Get Qubit` (`self.Character`) _returnvalue_x_2 _returnvalue_y))
        (set `/Game/Blueprints/BP_Board.Target` _qubit_2 _board_2)
        (`/Game/Blueprints/BP_Board.Normal Move` _board_2)
        (`self.K2_SetActorLocation` (`/Game/Blueprints/GlobalBP/Player+.Selected Piece` (`self.Character`)) (`KismetMathLibrary.MakeVector` _returnvalue_x_2 _returnvalue_y 60.0) false false)
        (`/Game/Blueprints/GlobalBP/Player+.ChangeTurns` (`self.Character`))
        (else
          (bind _qubit_3 (`/Game/Blueprints/GlobalBP/Player+.Get Qubit` (`self.Character`) _returnvalue_x_3 _returnvalue_y_2))
          (set `/Game/Blueprints/BP_Board.Measure` _qubit_3 _board)
          (`/Game/Blueprints/BP_Board.Measurement` _board)
          (if (`/Game/Blueprints/BP_Board.MeasurementResult` _board)
            (goto _label)
            (else
              (`/Game/Blueprints/GlobalBP/Player+.ChangeTurns` (`self.Character`))))))
      (else
        (goto _label_2)))
    (else
      (goto _label_2))))

(fn `UserConstructionScript`
  (bind _returnvalue (`self.K2_GetActorLocation`))
  (bind (_outhit _returnvalue_2) (`KismetSystemLibrary.LineTraceSingle` _returnvalue (+ _returnvalue (* (`self.GetActorUpVector`) -50.0)) "TraceTypeQuery1"))
  (if _returnvalue_2
    _
    (elif (`KismetSystemLibrary.IsValid` self)
      (`self.K2_DestroyActor`))))